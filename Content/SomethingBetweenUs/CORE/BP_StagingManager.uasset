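; Staging manager that advances the game through narrative stages, from title screen to epilogue, based on the Clean flags of BP_HeroAsset actors.
; Hero assets are sorted by name at BeginPlay and mapped to their flags, with only title and exposition assets visible.
; Each left click refreshes the map and tests hardcoded indices to set the stage.
; Middle stages cumulatively reveal assets by StageSpawn; Epilogue sets a post-process highlight parameter.
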(event EventBeginPlay
  (Variables|Default|SetCurrentStage "NewEnumerator0")
  (Input|EnableInput (Game|GetPlayerController 0))
  (bind _outactors (Actor|GetAllActorsOfClass "/Game/SomethingBetweenUs/HeroAssets/BP_HeroAsset.BP_HeroAsset_C"))
  ;[1 1 1] Put Hero Assets In Order
  (Utilities|Array|Sort _outactors true "Name")
  (for _array_element _outactors
    _)
  ;[1 1 1] Initialize Map
  (for _array_element_2 _outactors
    (Utilities|Map|Add (Variables|Default|GetHeroAssetMap_Clean) _array_element_2 (Variables|/Game/SomethingBetweenUs/HeroAssets/BP_HeroAsset.BP_HeroAsset_C|Getclean _array_element_2))
    ;[1 1 1] Setup Unlockable Objects
    (bind _keys (Utilities|Map|Keys (Variables|Default|GetHeroAssetMap_Clean)))
    (for _array_element_3 _keys
      (Rendering|SetActorHiddenInGame _array_element_3 (not (or (Utilities|Enum|Equal(Enum) (Variables|/Game/SomethingBetweenUs/HeroAssets/BP_HeroAsset.BP_HeroAsset_C|GetstageSpawn _array_element_3) "NewEnumerator0") (Utilities|Enum|Equal(Enum) (Variables|/Game/SomethingBetweenUs/HeroAssets/BP_HeroAsset.BP_HeroAsset_C|GetstageSpawn _array_element_3) "NewEnumerator1"))))
      (Development|PrintString (Utilities|String|ToString(Boolean) (not (or (Utilities|Enum|Equal(Enum) (Variables|/Game/SomethingBetweenUs/HeroAssets/BP_HeroAsset.BP_HeroAsset_C|GetstageSpawn _array_element_3) "NewEnumerator0") (Utilities|Enum|Equal(Enum) (Variables|/Game/SomethingBetweenUs/HeroAssets/BP_HeroAsset.BP_HeroAsset_C|GetstageSpawn _array_element_3) "NewEnumerator1")))) false))))

(event Input|MouseEvents|LeftMouseButton
  (params (Key :type Key%20Structure :default "None"))
  (:Pressed
    ;[1 1 1] Make Hero Asset Map
    (for _array_element (stale EventBeginPlay _outactors)
      (Utilities|Map|Add (Variables|Default|GetHeroAssetMap_Clean) _array_element (Variables|/Game/SomethingBetweenUs/HeroAssets/BP_HeroAsset.BP_HeroAsset_C|Getclean _array_element)))
    ;[1 1 1] Staging Switcher
    (bind _values (Utilities|Map|Values (Variables|Default|GetHeroAssetMap_Clean)))
    (Utilities|FlowControl|Sequence
      (:then_0
        (if (not (Utilities|Array|Get(acopy) _values (- 1 1)))
          (Variables|Default|SetCurrentStage "NewEnumerator1")))
      (:then_1
        (if (not (or (Utilities|Array|Get(acopy) _values (- 4 1)) (Utilities|Array|Get(acopy) _values (- 11 1))))
          (Variables|Default|SetCurrentStage "NewEnumerator2")))
      (:then_2
        (if (not (or (Utilities|Array|Get(acopy) _values (- 16 1)) (Utilities|Array|Get(acopy) _values (- 17 1))))
          (Variables|Default|SetCurrentStage "NewEnumerator3")))
      (:then_3
        (if (not (Utilities|Array|Get(acopy) _values (- 18 1)))
          (Variables|Default|SetCurrentStage "NewEnumerator4")))
      (:then_4
        (if (not (or (Utilities|Array|Get(acopy) _values (- 19 1)) (Utilities|Array|Get(acopy) _values (- 20 1))))
          (Variables|Default|SetCurrentStage "NewEnumerator5")))
      (:then_5
        (Development|PrintString (Utilities|String|EnumtoString (Variables|Default|GetCurrentStage)))
        (switch Utilities|FlowControl|Switch|SwitchonE_Stages (Variables|Default|GetCurrentStage)
          (:NewEnumerator2
            (bind _keys (Utilities|Map|Keys (Variables|Default|GetHeroAssetMap_Clean)))
            (for _array_element_2 _keys
              (Rendering|SetActorHiddenInGame _array_element_2 (not (Math|Boolean|ORBoolean (Utilities|Enum|Equal(Enum) (Variables|/Game/SomethingBetweenUs/HeroAssets/BP_HeroAsset.BP_HeroAsset_C|GetstageSpawn _array_element_2) "NewEnumerator0") (Utilities|Enum|Equal(Enum) (Variables|/Game/SomethingBetweenUs/HeroAssets/BP_HeroAsset.BP_HeroAsset_C|GetstageSpawn _array_element_2) "NewEnumerator1") (Utilities|Enum|Equal(Enum) (Variables|/Game/SomethingBetweenUs/HeroAssets/BP_HeroAsset.BP_HeroAsset_C|GetstageSpawn _array_element_2) "NewEnumerator2"))))))
          (:NewEnumerator3
            (bind _keys_2 (Utilities|Map|Keys (Variables|Default|GetHeroAssetMap_Clean)))
            (for _array_element_3 _keys_2
              (Rendering|SetActorHiddenInGame _array_element_3 (not (Math|Boolean|ORBoolean (Utilities|Enum|Equal(Enum) (Variables|/Game/SomethingBetweenUs/HeroAssets/BP_HeroAsset.BP_HeroAsset_C|GetstageSpawn _array_element_3) "NewEnumerator0") (Utilities|Enum|Equal(Enum) (Variables|/Game/SomethingBetweenUs/HeroAssets/BP_HeroAsset.BP_HeroAsset_C|GetstageSpawn _array_element_3) "NewEnumerator1") (Utilities|Enum|Equal(Enum) (Variables|/Game/SomethingBetweenUs/HeroAssets/BP_HeroAsset.BP_HeroAsset_C|GetstageSpawn _array_element_3) "NewEnumerator2") (Utilities|Enum|Equal(Enum) (Variables|/Game/SomethingBetweenUs/HeroAssets/BP_HeroAsset.BP_HeroAsset_C|GetstageSpawn _array_element_3) "NewEnumerator3"))))))
          (:NewEnumerator4
            (bind _keys_3 (Utilities|Map|Keys (Variables|Default|GetHeroAssetMap_Clean)))
            (for _array_element_4 _keys_3
              (Rendering|SetActorHiddenInGame _array_element_4 (not (Math|Boolean|ORBoolean (Utilities|Enum|Equal(Enum) (Variables|/Game/SomethingBetweenUs/HeroAssets/BP_HeroAsset.BP_HeroAsset_C|GetstageSpawn _array_element_4) "NewEnumerator0") (Utilities|Enum|Equal(Enum) (Variables|/Game/SomethingBetweenUs/HeroAssets/BP_HeroAsset.BP_HeroAsset_C|GetstageSpawn _array_element_4) "NewEnumerator1") (Utilities|Enum|Equal(Enum) (Variables|/Game/SomethingBetweenUs/HeroAssets/BP_HeroAsset.BP_HeroAsset_C|GetstageSpawn _array_element_4) "NewEnumerator2") (Utilities|Enum|Equal(Enum) (Variables|/Game/SomethingBetweenUs/HeroAssets/BP_HeroAsset.BP_HeroAsset_C|GetstageSpawn _array_element_4) "NewEnumerator3") (Utilities|Enum|Equal(Enum) (Variables|/Game/SomethingBetweenUs/HeroAssets/BP_HeroAsset.BP_HeroAsset_C|GetstageSpawn _array_element_4) "NewEnumerator4"))))))
          (:NewEnumerator5
            (Rendering|Material|SetScalarParameterValue "/Game/SomethingBetweenUs/CORE/MPC_PostProcess.MPC_PostProcess" "EpilogueHighlight?" 1.0 :!class /Script/Engine.KismetMaterialLibrary)))))))

(event Input|KeyboardEvents|H
  (params (Key :type Key%20Structure :default "None"))
  ;[1 1 1] Debug: Print Current Stage
  (:Pressed
    (Development|PrintString (Utilities|String|EnumtoString (Variables|Default|GetCurrentStage)))))

(fn ConstructionScript)