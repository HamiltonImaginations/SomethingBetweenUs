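; BP_HeroAsset is an interactive mesh actor that highlights under the cursor and triggers a camera move when clicked.
; Cursor enter and exit events switch an outline pass on its StaticMesh.
; A click clears the outline, runs ZoomOnClick on itself, then finds BP_CameraController with GetActorOfClass and invokes CallMoveToObject.
; On BeginPlay it stores the mesh asset's object name in Name.
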(event EventBeginPlay
  (Variables|Default|SetName (Utilities|GetObjectName (Variables|/Script/Engine.StaticMeshComponent|GetStaticMesh (Variables|Default|GetStaticMesh)))))

(event MouseInput|EventActorBeginCursorOver
  (CallFunction|ToggleOutlinePass true (Variables|Default|GetStaticMesh)))

(event MouseInput|EventActorEndCursorOver
  (CallFunction|ToggleOutlinePass false (Variables|Default|GetStaticMesh)))

(event MouseInput|EventActorOnClicked
  (params (ButtonPressed :type Key%20Structure :default "None"))
  (CallFunction|ToggleOutlinePass false (Variables|Default|GetStaticMesh))
  (CallFunction|ZoomonClick self)
  (bind _returnvalue (Actor|GetActorOfClass "/Game/SomethingBetweenUs/CORE/BP_CameraController.BP_CameraController_C"))
  (Default|CallMovetoObject _returnvalue))

(fn ConstructionScript)