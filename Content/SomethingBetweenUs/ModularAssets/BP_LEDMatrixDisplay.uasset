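; LED matrix display actor that slides two point lights along their relative X axis, apparently as a travelling glow for the display.
; On BeginPlay it caches the first light's relative location, then a timeline drives that light's X offset over a fixed travel distance.
; A second timeline starts after a delay and moves the second light the same way, also based on the first light's cached location.
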(event EventBeginPlay
  (Utilities|FlowControl|Sequence
    (:then_0
      (Variables|Default|SetLightLocation (Variables|/Script/Engine.SceneComponent|GetRelativeLocation (Variables|Default|GetPointLight))))
    (:then_1
      (bind _distancetotravel (Timeline|Timeline_0 Play)
        (:Update
          (Transformation|SetRelativeLocation (Variables|Default|GetPointLight) (Math|Vector|MakeVector (+ (.x (Variables|Default|GetLightLocation)) (* _distancetotravel 2.8e+02)) (.y (Variables|Default|GetLightLocation)) (.z (Variables|Default|GetLightLocation))) false false))))
    (:then_2
      (Utilities|FlowControl|Delay 1e+01)
      (bind _distancetotravel_2 (Timeline|Timeline_1 Play)
        (:Update
          (Transformation|SetRelativeLocation (Variables|Default|GetPointLight1) (Math|Vector|MakeVector (+ (.x (Variables|Default|GetLightLocation)) (* _distancetotravel_2 2.8e+02)) (.y (Variables|Default|GetLightLocation)) (.z (Variables|Default|GetLightLocation))) false false))))))

(event Collision|EventActorBeginOverlap
  (params (OtherActor :type Actor%20Object%20Reference)))

(event EventTick
  (params (DeltaSeconds :type Float%20%28single-precision%29)))

(fn ConstructionScript)